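; Projectile manager that renders nearby bullets, plays impact effects and supplies static humidity, pressure and wind values.
; BeginPlay pre-spawns Niagara and decal actor pools, which ApplyVFX cycles through round-robin when AsyncSim is off.
; Impacts choose sounds and decal materials by surface type, attaching decals to hit actors.
; While ShowBullets is on, Tick feeds positions, directions and mesh indices of bullets near the player into the pawn's Niagara component as arrays.
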(event `self.ReceiveBeginPlay`
  (`self.CreateVFXPools`))

(event `self.ReceiveTick`
  (params (DeltaSeconds :type "Float (single-precision)"))
  (if (`self.bShowBullets`)
    (`self.SetNiagaraParameters`)))

(event `self.ApplyVFX`
  (params (shouldSpawnDecal :type Boolean) (hitData :type "HitResult Structure (by ref)"))
  (bind (_bblockinghit _binitialoverlap _time _distance _location _impactpoint _normal) (`GameplayStatics.BreakHitResult` hitData))
  (bind (_bblockinghit_2 _binitialoverlap_2 _time_2 _distance_2 _location_2 _impactpoint_2 _normal_2 _impactnormal _physmat _hitactor) (`GameplayStatics.BreakHitResult` hitData))
  (bind _output (`|GetArrayItem` (`self.NiagaraActorsPool`) (`self.ParticleCount`)))
  (bind _output_2 (`|GetArrayItem` (`self.DecalActorsPool`) (`self.DecalCount`)))
  (bind _surfacetype (`PhysicalMaterial.SurfaceType` _physmat))
  (bind _decal (`DecalActor.Decal` _output_2))
  (bind _niagaracomponent (`NiagaraActor.NiagaraComponent` _output))
  ;[1 0.1042 0.1042] Optimization Nightmare
  (if (not (`self.AsyncSim`))
    (`|ExecutionSequence`
      (:`then_0`
        ;;[1 1 1] Activate Particle effect on impact
        (`self.K2_SetActorTransform` _output (`KismetMathLibrary.MakeTransform` _location (`KismetMathLibrary.FindLookAtRotation` _location (+ _location _normal))) false false)
        (`NiagaraComponent.SetAsset` _niagaracomponent "/BulletSystem/VFX/Particles/VFX_BulletHit.VFX_BulletHit" true)
        (`NiagaraComponent.ResetSystem` _niagaracomponent)
        (bind _result (`/Engine/EditorBlueprintResources/StandardMacros.IncrementInt` (`self.ParticleCount`))
          (:`  `
            (if (>= _result (`self.ImpactParticlePoolSize`))
              (set `self.ParticleCount` 0)))))
      (:`then_1`
        ;;[1 1 1] Activate decal based on impacted material if bullet was stopped
        (if shouldSpawnDecal
          (`self.K2_SetActorTransform` _output_2 (`KismetMathLibrary.MakeTransform` _location_2 (`KismetMathLibrary.FindLookAtRotation` _location_2 (- _location_2 _normal_2))) false false)
          (`self.K2_AttachToActor` _output_2 _hitactor "None" "KeepWorld" "KeepWorld" "KeepWorld" false)
          (`DecalComponent.SetDecalMaterial` _decal (select `EPhysicalSurface` _surfacetype :`SurfaceType_Default` "/BulletSystem/VFX/Decals/M_BulletDecal.M_BulletDecal" :`SurfaceType1` "/BulletSystem/VFX/Decals/MI_BulletDecalMetal.MI_BulletDecalMetal" :!type "MaterialInterface Object Reference"))
          (`SceneComponent.SetRelativeScale3D` _decal (/ 10.0 (`DecalComponent.DecalSize` _decal) (`self.GetActorScale3D` _hitactor)))
          (`DecalComponent.SetFadeScreenSize` _decal 0.005)
          (`SceneComponent.SetVisibility` _decal true false)
          (`GameplayStatics.PlaySoundAtLocation` (select `EPhysicalSurface` _surfacetype :`SurfaceType_Default` "/BulletSystem/Audio/BulletImpacts/SFX_BulletImpact_DEBUG.SFX_BulletImpact_DEBUG" :`SurfaceType1` "/Engine/VREditor/Sounds/UI/Foliage_Placed.Foliage_Placed" :!type "SoundBase Object Reference") _location_2 (struct) 1.0 1.0 0.0 "/BulletSystem/Audio/TestAttenuation.TestAttenuation" null null null)
          (bind _result_2 (`/Engine/EditorBlueprintResources/StandardMacros.IncrementInt` (`self.DecalCount`))
            (:`  `
              (if (>= _result_2 (`self.ImpactDecalPoolSize`))
                (set `self.DecalCount` 0))))
          (else
            (`GameplayStatics.PlaySoundAtLocation` (select `EPhysicalSurface` _surfacetype :`SurfaceType_Default` "/BulletSystem/Audio/BulletRicochets/SFX_BulletRicochet_DEBUG.SFX_BulletRicochet_DEBUG" :`SurfaceType1` "/Engine/VREditor/Sounds/UI/Click_on_Button_Cue.Click_on_Button_Cue" :!type "SoundBase Object Reference") _location_2 (struct) 1.0 1.0 0.0 "/BulletSystem/Audio/TestAttenuation.TestAttenuation" null null null)))))))

(fn `CreateVFXPools`
  (bind _returnvalue (`KismetMathLibrary.MakeTransform` (0.0 0.0 0.0)))
  (bind _niagaraactorspool (`self.NiagaraActorsPool`))
  (bind _decalactorspool (`self.DecalActorsPool`))
  (`|ExecutionSequence`
    (:`then_0`
      (`KismetArrayLibrary.Array_Resize` _niagaraactorspool (`self.ImpactParticlePoolSize`))
      (for (_ _array_index) _niagaraactorspool
        (bind _returnvalue_2 (`|SpawnActorFromClass` "/Script/Niagara.NiagaraActor" _returnvalue "Undefined" "MultiplyWithRoot" null null))
        (`KismetArrayLibrary.Array_Set` (`self.NiagaraActorsPool`) _array_index _returnvalue_2)))
    (:`then_1`
      (`KismetArrayLibrary.Array_Resize` _decalactorspool (`self.ImpactDecalPoolSize`))
      (for (_ _array_index_2) _decalactorspool
        (bind _returnvalue_3 (`|SpawnActorFromClass` "/Script/Engine.DecalActor" _returnvalue "Undefined" "MultiplyWithRoot" null null))
        (`KismetArrayLibrary.Array_Set` (`self.DecalActorsPool`) _array_index_2 _returnvalue_3)
        (`SceneComponent.SetVisibility` (`DecalActor.Decal` _returnvalue_3) false false)))))

(fn `GetHumidity`
  (params (location :type "Vector Structure (by ref)"))
  (returns (ReturnValue :type "Float (single-precision)"))
  (return (`StaticAtmosphereConditions.Humidity` (`self.StaticAtmosphericConditions`))))

(fn `GetPressure`
  (params (location :type "Vector Structure (by ref)"))
  (returns (ReturnValue :type "Float (single-precision)"))
  (return (`StaticAtmosphereConditions.Pressure` (`self.StaticAtmosphericConditions`))))

(fn `GetWind`
  (params (location :type "Vector Structure (by ref)"))
  (returns (ReturnValue :type "Vector Structure"))
  (return (`StaticAtmosphereConditions.Wind` (`self.StaticAtmosphericConditions`))))

(fn `SetNiagaraParameters`
  (locals (Positions :type "Array of Vector Structure") (Directions :type "Array of Vector Structure") (MeshIndeces :type "Array of Integer") (NearBullets :type "Array of Bullet Structure"))
  (bind _nearbullets (`local.NearBullets`))
  (bind _positions (`local.Positions`))
  (bind _returnvalue (`KismetArrayLibrary.Array_Length` _nearbullets))
  (bind _returnvalue_2 (`self.GetComponentByClass` (`GameplayStatics.GetPlayerPawn` 0) "/Script/Niagara.NiagaraComponent"))
  (for _array_element (`self.BulletList`)
    (if (< (`KismetMathLibrary.Vector_Distance` (`.StaritngPosition` (break `Bullet` _array_element)) (`self.K2_GetActorLocation` (`GameplayStatics.GetPlayerPawn` 0))) 500.0)
      (`KismetArrayLibrary.Array_Add` (`local.NearBullets`) _array_element)))
  (`KismetArrayLibrary.Array_Resize` (`local.Positions`) _returnvalue)
  (`KismetArrayLibrary.Array_Resize` (`local.Directions`) _returnvalue)
  (`KismetArrayLibrary.Array_Resize` (`local.MeshIndeces`) _returnvalue)
  (for (_array_element_2 _array_index) _nearbullets
    (bind (_staritngposition _direction _bulletdata) (break `Bullet` _array_element_2))
    (`KismetArrayLibrary.Array_Set` (`local.Positions`) _array_index _staritngposition)
    (`KismetArrayLibrary.Array_Set` (`local.Directions`) _array_index (`KismetMathLibrary.Normal` _direction))
    (`KismetArrayLibrary.Array_Set` (`local.MeshIndeces`) _array_index (`BlueprintMapLibrary.Map_Find` (`self.BulletMeshMap`) (`BulletType.BulletMesh` _bulletdata))))
  (`NiagaraDataInterfaceArrayFunctionLibrary.SetNiagaraArrayPosition` _returnvalue_2 "BulletPositions" _positions)
  (`NiagaraDataInterfaceArrayFunctionLibrary.SetNiagaraArrayPosition` _returnvalue_2 "TrailPositions" _positions)
  (`NiagaraDataInterfaceArrayFunctionLibrary.SetNiagaraArrayVector` _returnvalue_2 "BulletDirections" (`local.Directions`))
  (`NiagaraDataInterfaceArrayFunctionLibrary.SetNiagaraArrayInt32` _returnvalue_2 "BulletMeshes" (`local.MeshIndeces`)))

(fn `UserConstructionScript`)