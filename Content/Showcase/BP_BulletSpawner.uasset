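; BP_BulletSpawner is a showcase actor meant to fire example bullets along its Arrow component.
; Its loop passes CreateBullet the first player controller and a bullet built from the actor location, arrow forward times BulletSpeed, and DA_ExempleBullet.
; A Delay wired back into the call would repeat it ten times a second.
; The loop is not connected to BeginPlay or any other event, so nothing fires as it stands.
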(event `self.ReceiveBeginPlay`)

(fn `UserConstructionScript`)