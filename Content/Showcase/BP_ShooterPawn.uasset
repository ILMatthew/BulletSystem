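; Showcase shooter pawn that fires data-driven bullets from the player camera's aim on left mouse click.
; Each click passes start position, velocity and a bullet data asset to CreateBullet, with the controller as caller.
; HasShotGun selects a burst of randomly spread pellets within a cone, all sharing one data asset.
; Otherwise it fires one straight shot, alternating between two data assets as BulletType flips on every click.
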(event `Key|LeftMouseButton`
  (params (Key :type "Key Structure"))
  (bind _returnvalue (`SceneComponent.GetForwardVector` (`PlayerCameraManager.TransformComponent` (`GameplayStatics.GetPlayerCameraManager` 0))))
  (bind _returnvalue_2 (+ (`self.K2_GetActorLocation`) (* _returnvalue 60.0)))
  (:`Pressed`
    (set `self.bBulletType` (not (`self.bBulletType`)))
    (if (`self.bHasShotGun`)
      (for _ (range 8)
        (`ProjectilesManager.CreateBullet` (`self.GetController`) (make `Bullet` _returnvalue_2 (* (`KismetMathLibrary.RandomUnitVectorInConeInDegrees` _returnvalue (`self.ShotGunAngle`)) (`self.BulletSpeed`)) "/BulletSystem/Blueprints/BulletsData/DA_ExempleBullet1.DA_ExempleBullet1")))
      (else
        (`ProjectilesManager.CreateBullet` (`self.GetController`) (make `Bullet` _returnvalue_2 (* _returnvalue (`self.BulletSpeed`)) (select `bool` (`self.bBulletType`) :`false` "/BulletSystem/Blueprints/BulletsData/DA_ExempleBullet.DA_ExempleBullet" :`true` "/BulletSystem/Blueprints/BulletsData/DA_ExempleBullet1.DA_ExempleBullet1" :!type "BulletType Object Reference")))))))

(fn `UserConstructionScript`)