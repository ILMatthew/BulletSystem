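; Showcase actor demonstrating custom bullet-hit logic, with a health value shown through the color of its cube.
; On BeginPlay it fills Health and gives the cube a green dynamic debug material.
; Each Bullet event subtracts the bullet's Direction length times its Weight, clamps Health, and lerps the color toward red as it drops.
; ShouldBlockBullet always returns true, so the actor reports that it blocks every bullet.
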(event `self.ReceiveBeginPlay`
  (set `self.Health` (`self.MaxHealth`))
  (bind _returnvalue (`KismetMaterialLibrary.CreateDynamicMaterialInstance` "/PhysicVolumes/Materials/M_DebugSimpleColor.M_DebugSimpleColor"))
  (bind _output_get (set `self.DebugHealth` _returnvalue))
  (`PrimitiveComponent.SetMaterial` (`self.Cube`) 0 _output_get)
  (`MaterialInstanceDynamic.SetVectorParameterValue` _output_get "Color" (struct :`R` 0.206092 :`G` 1.0 :`A` 1.0)))

(event `self.ReceiveBullet`
  (params (bullet :type "Bullet Structure (by ref)") (hitBone :type Name))
  (bind (_staritngposition _direction _bulletdata) (break `Bullet` bullet))
  (bind _maxhealth (`self.MaxHealth`))
  ;[0.5235 1 0] Exemple Health reduction based on bullet stats
  (bind _output_get (set `self.Health` (`KismetMathLibrary.FClamp` (- (`self.Health`) (* (`KismetMathLibrary.VSize` _direction) (`BulletType.Weight` _bulletdata))) 0.0 _maxhealth)))
  (`MaterialInstanceDynamic.SetVectorParameterValue` (`self.DebugHealth`) "Color" (`KismetMathLibrary.LinearColorLerp` (struct :`R` 1.0 :`B` 0.016807 :`A` 1.0) (struct :`R` 0.205079 :`G` 1.0 :`A` 1.0) (/ _output_get _maxhealth))))

(fn `ShouldBlockBullet`
  (returns (ReturnValue :type Boolean))
  (return true))

(fn `UserConstructionScript`)